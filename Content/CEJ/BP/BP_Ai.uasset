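; BP_Ai is an AI pawn that wanders, then chases and attacks the first BP_BouncyBall found at BeginPlay.
; AiRoam loops AIMoveTo on random reachable points.
; Any PawnSensing sighting raises walk speed and moves it to that cached ball, triggering a DoOnce-gated montage attack on arrival.
; CanAttack is never cleared, and a disconnected branch holds an unused delayed return to slower roaming.
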(event `self.ReceiveBeginPlay`
  (bind _outactors (`GameplayStatics.GetAllActorsOfClass` "/Game/OSC/BluePrints/BP_BouncyBall.BP_BouncyBall_C"))
  (set `self.TargetName` (`|GetArrayItem` _outactors))
  (`PrimitiveComponent.SetCollisionResponseToChannel` (`self.Mesh`) "ECC_Camera" "ECR_Ignore")
  (`self.AiRoam`))

(event `AiRoam`
  ; random move
  (`|AIMoveTo` self (`NavigationSystemV1.K2_GetRandomReachablePointInRadius` (`self.K2_GetActorLocation`) 1500.0 null null) null
    (:`OnSuccess`
      (`KismetSystemLibrary.Delay` 0.2)
      (`self.AiRoam`))))

(event `self.PawnSensing.OnSeePawn`
  (params (Pawn :type "Pawn Object Reference"))
  ; random move
  (set `self.CanAttack` true)
  (set `CharacterMovementComponent.MaxWalkSpeed` 600.0 (`self.CharacterMovement`))
  (`|AIMoveTo` self (0.0 0.0 0.0) (`self.TargetName`) 70.0
    (:`OnSuccess`
      (if (`self.CanAttack`)
        (set `self.CanAttack` true)
        (`self.Attack`)))))

(event `Attack`
  (`/Engine/EditorBlueprintResources/StandardMacros.DoOnce` false :!label _label
    (:`Completed`
      (bind _returnvalue (`self.PlayAnimMontage` self null 1.0 "None"))
      (`KismetSystemLibrary.Delay` _returnvalue)
      (set `self.CanAttack` true)
      (goto _label :!via `Reset`))))

(fn `UserConstructionScript`)