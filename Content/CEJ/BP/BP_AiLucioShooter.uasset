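; BP_AiLucioShooter is an AI character that moves toward the Ball and attempts to knock it away, once, at BeginPlay.
; It issues AI MoveTo with a wide acceptance radius, then runs a debug-drawn, zero-length sphere trace ahead of its mesh from the immediate Then output, without waiting for arrival.
; A BP_BouncyBall hit receives a forward-and-upward impulse through BouncyBallAddImpulse, with this actor as attacker.
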(event `self.ReceiveBeginPlay`
  (bind _returnvalue (+ (`SceneComponent.K2_GetComponentLocation` (`self.Mesh`)) (* (`SceneComponent.GetForwardVector` (`self.Mesh`)) 150.0)))
  (`|AIMoveTo` self (0.0 0.0 0.0) (`self.ball`) 3000.0
    (:`then`
      (bind _outhit (`KismetSystemLibrary.SphereTraceSingleForObjects` :`Start` _returnvalue :`End` _returnvalue :`Radius` 100.0 :`ObjectTypes` (`|MakeArray` "ObjectTypeQuery7" :!type "EObjectTypeQuery Enum") :`DrawDebugType` "ForDuration"))
      (bind _asbp_bouncy_ball (cast `/Game/OSC/BluePrints/BP_BouncyBall` (`.HitActor` (`GameplayStatics.BreakHitResult` _outhit))))
      (`BouncyBall.BouncyBallAddImpulse` _asbp_bouncy_ball (* (`KismetMathLibrary.Normal` (+ (`self.GetActorForwardVector`) (0.0 0.0 1.0))) 1000.0) self))))

(fn `UserConstructionScript`)