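; Firework launcher actor that fires a timed series of BP_Rocket_Single rockets from Example_DataTable, then destroys itself.
; AddData reads a row in table order, or at random with IsRandom, clamps most numeric settings and calls Launch with the row's delay.
; Launch spawns a rocket at the root or within an optional bounding box, copies the settings across and fires it next tick.
; It then calls AddData again, chaining launches for the table's row count.
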(event `self.ReceiveBeginPlay`
  ;[1 1 1] Add new data to rocket and launch
  ;;[1 1 1] Gets row data
  (`self.AddData` 0)
  (if (`self.IsRandom`)
    (bind _outrownames (`DataTableFunctionLibrary.GetDataTableRowNames` "/Game/ModularFireworks2/Example_DataTable.Example_DataTable"))
    (set `self.Row` (`KismetArrayLibrary.Array_Length` _outrownames))))

(event `launch`
  (params (Delay :type "Float (double-precision)"))
  (bind _row (`self.Row`))
  (bind _box (`self.Box`))
  (bind _row_2 (`self.Row`))
  (bind (_returnvalue_location _returnvalue_rotation _returnvalue_scale) (`KismetMathLibrary.BreakTransform` (`SceneComponent.K2_GetComponentToWorld` (`self.DefaultSceneRoot`))))
  ;[1 1 1] Add new data to rocket and launch
  (`KismetSystemLibrary.Delay` Delay)
  (if (`self.Use Bounding Box`)
    (set `self.SpawnTransform` (`KismetMathLibrary.MakeTransform` (`KismetMathLibrary.RandomPointInBoundingBox` (`SceneComponent.K2_GetComponentLocation` _box) (`BoxComponent.GetScaledBoxExtent` _box)) _returnvalue_rotation _returnvalue_scale))
    (else
      (set `self.SpawnTransform` (`SceneComponent.K2_GetComponentToWorld` (`self.DefaultSceneRoot`)))))
  (bind _returnvalue (`|SpawnActorFromClass` "/Game/ModularFireworks2/BackEnd/DataTableBackend/BP_Rocket_Single.BP_Rocket_Single_C" (`self.SpawnTransform`) "Undefined" "MultiplyWithRoot" null null))
  (`|ExecutionSequence`
    (:`then_0`
      (set `/Game/ModularFireworks2/BackEnd/DataTableBackend/BP_Rocket_Single.System` (`self.System`) _returnvalue))
    (:`then_1`
      (set `/Game/ModularFireworks2/BackEnd/DataTableBackend/BP_Rocket_Single.Colour` (`self.Colour`) _returnvalue))
    (:`then_2`
      (set `/Game/ModularFireworks2/BackEnd/DataTableBackend/BP_Rocket_Single.Does Scale Colour` (`self.Has Colour Variation`) _returnvalue))
    (:`then_3`
      (set `/Game/ModularFireworks2/BackEnd/DataTableBackend/BP_Rocket_Single.DoesRenderLight` (`self.DoesRenderLight`) _returnvalue))
    (:`then_4`
      (set `/Game/ModularFireworks2/BackEnd/DataTableBackend/BP_Rocket_Single.Brightness` (`self.Brightness`) _returnvalue))
    (:`then_5`
      (set `/Game/ModularFireworks2/BackEnd/DataTableBackend/BP_Rocket_Single.Number Of Particles` (`self.Number Of Particles`) _returnvalue))
    (:`then_6`
      (set `/Game/ModularFireworks2/BackEnd/DataTableBackend/BP_Rocket_Single.Size of explosion` (`self.Size`) _returnvalue))
    (:`then_7`
      (set `/Game/ModularFireworks2/BackEnd/DataTableBackend/BP_Rocket_Single.Has Smoke` (`self.Has Smoke`) _returnvalue))
    (:`then_8`
      (set `/Game/ModularFireworks2/BackEnd/DataTableBackend/BP_Rocket_Single.Smoke Lifetime` (`self.Smoke Lifetime`) _returnvalue))
    (:`then_9`
      (set `/Game/ModularFireworks2/BackEnd/DataTableBackend/BP_Rocket_Single.Smoke Size` (`self.Smoke Size`) _returnvalue))
    (:`then_10`
      (set `/Game/ModularFireworks2/BackEnd/DataTableBackend/BP_Rocket_Single.Smoke Amount` (`self.Smoke Amount`) _returnvalue))
    (:`then_11`
      (set `/Game/ModularFireworks2/BackEnd/DataTableBackend/BP_Rocket_Single.Speed` (`self.Speed`) _returnvalue))
    (:`then_12`
      (set `/Game/ModularFireworks2/BackEnd/DataTableBackend/BP_Rocket_Single.Distance` (`self.Distance`) _returnvalue))
    (:`then_13`
      (set `/Game/ModularFireworks2/BackEnd/DataTableBackend/BP_Rocket_Single.Explosion Sound` (`self.Explosion Sound`) _returnvalue))
    (:`then_14`
      (set `/Game/ModularFireworks2/BackEnd/DataTableBackend/BP_Rocket_Single.Volume Multiplier Explosion` (`self.Volume Multiplier Explosion`) _returnvalue))
    (:`then_15`
      (set `/Game/ModularFireworks2/BackEnd/DataTableBackend/BP_Rocket_Single.Whistle Sound` (`self.Whistle Sound`) _returnvalue))
    (:`then_16`
      (set `/Game/ModularFireworks2/BackEnd/DataTableBackend/BP_Rocket_Single.Volume Multiplier Whistle` (`self.Volume Multiplier Whistle`) _returnvalue))
    (:`then_17`
      (set `/Game/ModularFireworks2/BackEnd/DataTableBackend/BP_Rocket_Single.Trail Spawn Rate` (`self.Trail Spawn Rate`) _returnvalue))
    (:`then_18`
      (set `/Game/ModularFireworks2/BackEnd/DataTableBackend/BP_Rocket_Single.Does Match Explosion Colour` (`self.Does Match Explosion Colour`) _returnvalue))
    (:`then_19`
      (set `/Game/ModularFireworks2/BackEnd/DataTableBackend/BP_Rocket_Single.TrailColour` (`self.TrailColour`) _returnvalue))
    (:`then_20`
      (set `/Game/ModularFireworks2/BackEnd/DataTableBackend/BP_Rocket_Single.Does Render Light` (`self.Does Render Light`) _returnvalue))
    (:`then_21`
      (set `/Game/ModularFireworks2/BackEnd/DataTableBackend/BP_Rocket_Single.Has Trail Smoke` (`self.Has Trail Smoke`) _returnvalue))
    (:`then_22`
      (set `/Game/ModularFireworks2/BackEnd/DataTableBackend/BP_Rocket_Single.Trail Smoke Amount` (`self.Trail Smoke Amount`) _returnvalue))
    (:`then_23`
      (set `/Game/ModularFireworks2/BackEnd/DataTableBackend/BP_Rocket_Single.Trail Smoke Lifetime` (`self.Trail Smoke Lifetime`) _returnvalue))
    (:`then_24`
      (set `/Game/ModularFireworks2/BackEnd/DataTableBackend/BP_Rocket_Single.Scale Colour Amount` (`self.Colour Var Amount`) _returnvalue))
    (:`then_25`
      (set `/Game/ModularFireworks2/BackEnd/DataTableBackend/BP_Rocket_Single.Particle Size` (`self.Particle Size`) _returnvalue))
    (:`then_26`
      (set `/Game/ModularFireworks2/BackEnd/DataTableBackend/BP_Rocket_Single.Particle Lifetime` (`self.Particle Lifetime`) _returnvalue))
    (:`then_27`
      (set `/Game/ModularFireworks2/BackEnd/DataTableBackend/BP_Rocket_Single.Trail Length` (`self.Trail Length`) _returnvalue))
    (:`then_28`
      (`KismetSystemLibrary.DelayUntilNextTick`)
      (`/Game/ModularFireworks2/BackEnd/DataTableBackend/BP_Rocket_Single.LaunchSingle` _returnvalue)
      (if (`self.IsRandom`)
        (`/Engine/EditorBlueprintResources/StandardMacros.DecrementInt` _row_2
          (:`  `
            (if (<= _row_2 0)
              (`self.K2_DestroyActor`)
              (else
                (`self.AddData` 0)))))
        (else
          (bind _outrownames (`DataTableFunctionLibrary.GetDataTableRowNames` "/Game/ModularFireworks2/Example_DataTable.Example_DataTable"))
          (if (< _row (- (`KismetArrayLibrary.Array_Length` _outrownames) 1))
            (bind _result (`/Engine/EditorBlueprintResources/StandardMacros.IncrementInt` _row)
              (:`  `
                (`self.AddData` _result)))
            (else
              (`self.K2_DestroyActor`))))))))

(fn `AddData`
  (params (Row :type Integer))
  ;[1 1 1] Set variables in firework then launch and reset for next
  (if (`self.IsRandom`)
    (bind _outrownames (`DataTableFunctionLibrary.GetDataTableRowNames` "/Game/ModularFireworks2/Example_DataTable.Example_DataTable"))
    (bind _returnvalue (`|GetDataTableRow` "/Game/ModularFireworks2/Example_DataTable.Example_DataTable" (`KismetArrayLibrary.Array_Random` _outrownames))
      (:`then`
        (`|ExecutionSequence`
          (:`then_0`
            (set `self.System` (`.System_2_2912C69B4AC7968D5A6CCAB6F27C70B6` (break `/Game/ModularFireworks2/BackEnd/DataTableBackend/S_FireworkVariables` _returnvalue))))
          (:`then_1`
            (set `self.Colour` (`.ColourExplosion_12_2AEFA46C4F5B40F603BAF18E3F09B62E` (break `/Game/ModularFireworks2/BackEnd/DataTableBackend/S_FireworkVariables` _returnvalue))))
          (:`then_2`
            (set `self.Has Colour Variation` (`.HasScaleColour_82_817853EB4C8845C47AF4DC955F5CD72A` (break `/Game/ModularFireworks2/BackEnd/DataTableBackend/S_FireworkVariables` _returnvalue))))
          (:`then_3`
            (set `self.DoesRenderLight` false))
          (:`then_4`
            (set `self.Brightness` (`KismetMathLibrary.FClamp` (`.Brightness_25_4364372046C878E84BED25A8B28FF317` (break `/Game/ModularFireworks2/BackEnd/DataTableBackend/S_FireworkVariables` _returnvalue)) 0.0 50.0)))
          (:`then_5`
            (set `self.Number Of Particles` (`KismetMathLibrary.Clamp` (`.NumberOfParticles_26_83F7D62342869F600294F791E8E7B8BE` (break `/Game/ModularFireworks2/BackEnd/DataTableBackend/S_FireworkVariables` _returnvalue)) 0 10000)))
          (:`then_6`
            (set `self.Size` (`KismetMathLibrary.FClamp` (`.Sizeofexplosion_91_8D37DF294E7037AA7B98779A99542303` (break `/Game/ModularFireworks2/BackEnd/DataTableBackend/S_FireworkVariables` _returnvalue)) 0.0 50.0)))
          (:`then_7`
            (set `self.Has Smoke` (`.HasSmoke_29_92CDAC7E421ACF979166A183CF19D589` (break `/Game/ModularFireworks2/BackEnd/DataTableBackend/S_FireworkVariables` _returnvalue))))
          (:`then_8`
            (set `self.Smoke Lifetime` (`KismetMathLibrary.FClamp` (`.SmokeLifetime_36_9C0387B8491BCD25111F81980D79AE8C` (break `/Game/ModularFireworks2/BackEnd/DataTableBackend/S_FireworkVariables` _returnvalue)) 5.0 20.0)))
          (:`then_9`
            (set `self.Smoke Size` (`KismetMathLibrary.FClamp` (`.SmokeSize_37_2654059042C3CE60A7BB16AC335F511D` (break `/Game/ModularFireworks2/BackEnd/DataTableBackend/S_FireworkVariables` _returnvalue)) 0.1 10.0)))
          (:`then_10`
            (set `self.Smoke Amount` (`KismetMathLibrary.FClamp` (`.SmokeAmount_38_299B65BE49BA5D19B7F5179F9C9AAEC5` (break `/Game/ModularFireworks2/BackEnd/DataTableBackend/S_FireworkVariables` _returnvalue)) 0.1 10.0)))
          (:`then_11`
            (set `self.Speed` (`KismetMathLibrary.FClamp` (`.Speed_40_3F1A7A464CF6B0209E12A6B1AA26E176` (break `/Game/ModularFireworks2/BackEnd/DataTableBackend/S_FireworkVariables` _returnvalue)) 1.0 20.0)))
          (:`then_12`
            (set `self.Distance` (`KismetMathLibrary.FClamp` (`.Distance_79_C3689DC34CBDE7A044E6DB867F6EF204` (break `/Game/ModularFireworks2/BackEnd/DataTableBackend/S_FireworkVariables` _returnvalue)) 1.0 50.0)))
          (:`then_13`
            (set `self.Explosion Sound` (`.ExplosionSound_45_F488579D4D8AC3D3C21BBBB8E552FD5B` (break `/Game/ModularFireworks2/BackEnd/DataTableBackend/S_FireworkVariables` _returnvalue))))
          (:`then_14`
            (set `self.Volume Multiplier Explosion` (`.Volumeofexplosionsound_54_46E244D441071DAE713E08A0E92FFB1C` (break `/Game/ModularFireworks2/BackEnd/DataTableBackend/S_FireworkVariables` _returnvalue))))
          (:`then_15`
            (set `self.Whistle Sound` (`.Whistlestartsound_49_98A8CEEA481A6A2E046324A7B7E590A1` (break `/Game/ModularFireworks2/BackEnd/DataTableBackend/S_FireworkVariables` _returnvalue))))
          (:`then_16`
            (set `self.Volume Multiplier Whistle` (`.Volumeofstartsound_53_69A8B2B849B1D30E65F11394D22ECC78` (break `/Game/ModularFireworks2/BackEnd/DataTableBackend/S_FireworkVariables` _returnvalue))))
          (:`then_17`
            (set `self.Trail Spawn Rate` (`KismetMathLibrary.FClamp` (`.TrailSpawnRate_56_1F584F6841D62983B6FF69B4F7F081FB` (break `/Game/ModularFireworks2/BackEnd/DataTableBackend/S_FireworkVariables` _returnvalue)) 0.0 1000.0)))
          (:`then_18`
            (set `self.TrailColour` (`.TrailColour_63_0676E53945B2D58A91FF379089F171BF` (break `/Game/ModularFireworks2/BackEnd/DataTableBackend/S_FireworkVariables` _returnvalue))))
          (:`then_19`
            (set `self.Does Match Explosion Colour` (`.DoesMatchExplosioncolourtrailandexplosioncolourmatch_70_6AF410944A491C60E3EAB39D37AAAE91` (break `/Game/ModularFireworks2/BackEnd/DataTableBackend/S_FireworkVariables` _returnvalue))))
          (:`then_20`
            (set `self.Does Render Light` (`.DoesRenderLightTrail_64_194ED0E5417D2820AC8C8B8EA706DD60` (break `/Game/ModularFireworks2/BackEnd/DataTableBackend/S_FireworkVariables` _returnvalue))))
          (:`then_21`
            (set `self.Has Trail Smoke` (`.HasTrailSmoke_67_AEBC6EBE4D2D3EA300F26AB606445DEA` (break `/Game/ModularFireworks2/BackEnd/DataTableBackend/S_FireworkVariables` _returnvalue))))
          (:`then_22`
            (set `self.Trail Smoke Amount` (`KismetMathLibrary.FClamp` (`.TrailSmokeSpawnRate_81_2325F179471920DB5CE0E9B5E2777847` (break `/Game/ModularFireworks2/BackEnd/DataTableBackend/S_FireworkVariables` _returnvalue)) 0.0 1000.0)))
          (:`then_23`
            (set `self.Trail Smoke Lifetime` (`KismetMathLibrary.FClamp` (`.TrailSmokeLifetime_80_520A9E134BF3752CAD36ED930B7D9277` (break `/Game/ModularFireworks2/BackEnd/DataTableBackend/S_FireworkVariables` _returnvalue)) 5.0 20.0)))
          (:`then_24`
            (set `self.Colour Var Amount` (`KismetMathLibrary.FClamp` (`.ScaleColourAmount_85_0CC70A04416E70141F6D1CA4526A399D` (break `/Game/ModularFireworks2/BackEnd/DataTableBackend/S_FireworkVariables` _returnvalue)) 0.0 10.0)))
          (:`then_25`
            (set `self.Particle Size` (`KismetMathLibrary.FClamp` (`.ParticleSize_87_6EE0DE4846DCB5F83EA0949869C64282` (break `/Game/ModularFireworks2/BackEnd/DataTableBackend/S_FireworkVariables` _returnvalue)) 1.0 20.0)))
          (:`then_26`
            (set `self.Particle Lifetime` (`KismetMathLibrary.FClamp` (`.ParticleLifetime_90_3ACE569A4A655B56250D7C97A688984E` (break `/Game/ModularFireworks2/BackEnd/DataTableBackend/S_FireworkVariables` _returnvalue)) 1.0 10.0)))
          (:`then_27`
            (set `self.Trail Length` (`KismetMathLibrary.FClamp` (`.TrailLength_93_E0B55AF34DA6F93CFCE2AE88A9C2D1A4` (break `/Game/ModularFireworks2/BackEnd/DataTableBackend/S_FireworkVariables` _returnvalue)) 0.0 3.0)))
          (:`then_28`
            (`self.launch` (break `/Game/ModularFireworks2/BackEnd/DataTableBackend/S_FireworkVariables` _returnvalue)))))
      (:`RowNotFound`
        (`self.K2_DestroyActor`)))
    (else
      (bind _outrownames_2 (`DataTableFunctionLibrary.GetDataTableRowNames` "/Game/ModularFireworks2/Example_DataTable.Example_DataTable"))
      (bind _returnvalue_2 (`|GetDataTableRow` "/Game/ModularFireworks2/Example_DataTable.Example_DataTable" (`|GetArrayItem` _outrownames_2 Row))
        (:`then`
          (`|ExecutionSequence`
            (:`then_0`
              (set `self.System` (`.System_2_2912C69B4AC7968D5A6CCAB6F27C70B6` (break `/Game/ModularFireworks2/BackEnd/DataTableBackend/S_FireworkVariables` _returnvalue_2))))
            (:`then_1`
              (set `self.Colour` (`.ColourExplosion_12_2AEFA46C4F5B40F603BAF18E3F09B62E` (break `/Game/ModularFireworks2/BackEnd/DataTableBackend/S_FireworkVariables` _returnvalue_2))))
            (:`then_2`
              (set `self.Has Colour Variation` (`.HasScaleColour_82_817853EB4C8845C47AF4DC955F5CD72A` (break `/Game/ModularFireworks2/BackEnd/DataTableBackend/S_FireworkVariables` _returnvalue_2))))
            (:`then_3`
              (set `self.DoesRenderLight` false))
            (:`then_4`
              (set `self.Brightness` (`KismetMathLibrary.FClamp` (`.Brightness_25_4364372046C878E84BED25A8B28FF317` (break `/Game/ModularFireworks2/BackEnd/DataTableBackend/S_FireworkVariables` _returnvalue_2)) 0.0 50.0)))
            (:`then_5`
              (set `self.Number Of Particles` (`KismetMathLibrary.Clamp` (`.NumberOfParticles_26_83F7D62342869F600294F791E8E7B8BE` (break `/Game/ModularFireworks2/BackEnd/DataTableBackend/S_FireworkVariables` _returnvalue_2)) 0 10000)))
            (:`then_6`
              (set `self.Size` (`KismetMathLibrary.FClamp` (`.Sizeofexplosion_91_8D37DF294E7037AA7B98779A99542303` (break `/Game/ModularFireworks2/BackEnd/DataTableBackend/S_FireworkVariables` _returnvalue_2)) 0.0 50.0)))
            (:`then_7`
              (set `self.Has Smoke` (`.HasSmoke_29_92CDAC7E421ACF979166A183CF19D589` (break `/Game/ModularFireworks2/BackEnd/DataTableBackend/S_FireworkVariables` _returnvalue_2))))
            (:`then_8`
              (set `self.Smoke Lifetime` (`KismetMathLibrary.FClamp` (`.SmokeLifetime_36_9C0387B8491BCD25111F81980D79AE8C` (break `/Game/ModularFireworks2/BackEnd/DataTableBackend/S_FireworkVariables` _returnvalue_2)) 5.0 20.0)))
            (:`then_9`
              (set `self.Smoke Size` (`KismetMathLibrary.FClamp` (`.SmokeSize_37_2654059042C3CE60A7BB16AC335F511D` (break `/Game/ModularFireworks2/BackEnd/DataTableBackend/S_FireworkVariables` _returnvalue_2)) 0.1 10.0)))
            (:`then_10`
              (set `self.Smoke Amount` (`KismetMathLibrary.FClamp` (`.SmokeAmount_38_299B65BE49BA5D19B7F5179F9C9AAEC5` (break `/Game/ModularFireworks2/BackEnd/DataTableBackend/S_FireworkVariables` _returnvalue_2)) 0.1 10.0)))
            (:`then_11`
              (set `self.Speed` (`KismetMathLibrary.FClamp` (`.Speed_40_3F1A7A464CF6B0209E12A6B1AA26E176` (break `/Game/ModularFireworks2/BackEnd/DataTableBackend/S_FireworkVariables` _returnvalue_2)) 1.0 20.0)))
            (:`then_12`
              (set `self.Distance` (`KismetMathLibrary.FClamp` (`.Distance_79_C3689DC34CBDE7A044E6DB867F6EF204` (break `/Game/ModularFireworks2/BackEnd/DataTableBackend/S_FireworkVariables` _returnvalue_2)) 1.0 50.0)))
            (:`then_13`
              (set `self.Explosion Sound` (`.ExplosionSound_45_F488579D4D8AC3D3C21BBBB8E552FD5B` (break `/Game/ModularFireworks2/BackEnd/DataTableBackend/S_FireworkVariables` _returnvalue_2))))
            (:`then_14`
              (set `self.Volume Multiplier Explosion` (`.Volumeofexplosionsound_54_46E244D441071DAE713E08A0E92FFB1C` (break `/Game/ModularFireworks2/BackEnd/DataTableBackend/S_FireworkVariables` _returnvalue_2))))
            (:`then_15`
              (set `self.Whistle Sound` (`.Whistlestartsound_49_98A8CEEA481A6A2E046324A7B7E590A1` (break `/Game/ModularFireworks2/BackEnd/DataTableBackend/S_FireworkVariables` _returnvalue_2))))
            (:`then_16`
              (set `self.Volume Multiplier Whistle` (`.Volumeofstartsound_53_69A8B2B849B1D30E65F11394D22ECC78` (break `/Game/ModularFireworks2/BackEnd/DataTableBackend/S_FireworkVariables` _returnvalue_2))))
            (:`then_17`
              (set `self.Trail Spawn Rate` (`KismetMathLibrary.FClamp` (`.TrailSpawnRate_56_1F584F6841D62983B6FF69B4F7F081FB` (break `/Game/ModularFireworks2/BackEnd/DataTableBackend/S_FireworkVariables` _returnvalue_2)) 0.0 1000.0)))
            (:`then_18`
              (set `self.TrailColour` (`.TrailColour_63_0676E53945B2D58A91FF379089F171BF` (break `/Game/ModularFireworks2/BackEnd/DataTableBackend/S_FireworkVariables` _returnvalue_2))))
            (:`then_19`
              (set `self.Does Match Explosion Colour` (`.DoesMatchExplosioncolourtrailandexplosioncolourmatch_70_6AF410944A491C60E3EAB39D37AAAE91` (break `/Game/ModularFireworks2/BackEnd/DataTableBackend/S_FireworkVariables` _returnvalue_2))))
            (:`then_20`
              (set `self.Does Render Light` (`.DoesRenderLightTrail_64_194ED0E5417D2820AC8C8B8EA706DD60` (break `/Game/ModularFireworks2/BackEnd/DataTableBackend/S_FireworkVariables` _returnvalue_2))))
            (:`then_21`
              (set `self.Has Trail Smoke` (`.HasTrailSmoke_67_AEBC6EBE4D2D3EA300F26AB606445DEA` (break `/Game/ModularFireworks2/BackEnd/DataTableBackend/S_FireworkVariables` _returnvalue_2))))
            (:`then_22`
              (set `self.Trail Smoke Amount` (`KismetMathLibrary.FClamp` (`.TrailSmokeSpawnRate_81_2325F179471920DB5CE0E9B5E2777847` (break `/Game/ModularFireworks2/BackEnd/DataTableBackend/S_FireworkVariables` _returnvalue_2)) 0.0 1000.0)))
            (:`then_23`
              (set `self.Trail Smoke Lifetime` (`KismetMathLibrary.FClamp` (`.TrailSmokeLifetime_80_520A9E134BF3752CAD36ED930B7D9277` (break `/Game/ModularFireworks2/BackEnd/DataTableBackend/S_FireworkVariables` _returnvalue_2)) 5.0 20.0)))
            (:`then_24`
              (set `self.Colour Var Amount` (`KismetMathLibrary.FClamp` (`.ScaleColourAmount_85_0CC70A04416E70141F6D1CA4526A399D` (break `/Game/ModularFireworks2/BackEnd/DataTableBackend/S_FireworkVariables` _returnvalue_2)) 0.0 10.0)))
            (:`then_25`
              (set `self.Particle Size` (`KismetMathLibrary.FClamp` (`.ParticleSize_87_6EE0DE4846DCB5F83EA0949869C64282` (break `/Game/ModularFireworks2/BackEnd/DataTableBackend/S_FireworkVariables` _returnvalue_2)) 1.0 20.0)))
            (:`then_26`
              (set `self.Particle Lifetime` (`KismetMathLibrary.FClamp` (`.ParticleLifetime_90_3ACE569A4A655B56250D7C97A688984E` (break `/Game/ModularFireworks2/BackEnd/DataTableBackend/S_FireworkVariables` _returnvalue_2)) 1.0 10.0)))
            (:`then_27`
              (set `self.Trail Length` (`KismetMathLibrary.FClamp` (`.TrailLength_93_E0B55AF34DA6F93CFCE2AE88A9C2D1A4` (break `/Game/ModularFireworks2/BackEnd/DataTableBackend/S_FireworkVariables` _returnvalue_2)) 0.0 3.0)))
            (:`then_28`
              (`self.launch` (break `/Game/ModularFireworks2/BackEnd/DataTableBackend/S_FireworkVariables` _returnvalue_2)))))
        (:`RowNotFound`
          (`self.K2_DestroyActor`))))))

(fn `UserConstructionScript`)