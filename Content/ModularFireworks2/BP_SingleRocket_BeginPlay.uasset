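; Single firework rocket actor that launches after a randomized delay, flies with a trail and whistle, then explodes and destroys itself once smoke lifetime ends.
; The construction script picks one of three peony Niagara systems and pushes colour, particle, light, smoke and trail settings into both effects.
; BeginPlay drives flight with a looping timer offset and spin, detonating after Distance/Speed.
; Separate events provide test bursts and random colours.
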(event `self.ReceiveBeginPlay`
  (bind _delay (`self.Delay`))
  (bind _smoke_lifetime (`self.Smoke Lifetime`))
  (bind _trail_smoke_lifetime (`self.Trail Smoke Lifetime`))
  (bind _delayvariation (`self.DelayVariation`))
  ;[1 1 1] Reset rocket (from test)
  (`SceneComponent.K2_SetWorldLocation` (`self.Niagara`) (`SceneComponent.K2_GetComponentLocation` (`self.Rocket`)) false false)
  ;[1 1 1] Delay before launch
  (`KismetSystemLibrary.Delay` (`KismetMathLibrary.FClamp` (+ _delay (`KismetMathLibrary.RandomFloatInRange` (* _delayvariation -1.0) _delayvariation)) 0.0 (+ _delay _delayvariation)))
  (`GameplayStatics.PlaySoundAtLocation` (`self.Whistle Sound`) (`self.K2_GetActorLocation`) (struct) (`self.Volume Multiplier Whistle`) (`KismetMathLibrary.RandomFloatInRange` 0.7 1.3) 0.0 "/Game/ModularFireworks2/BackEnd/Niagara/Sound/Att_Firework.Att_Firework" null null null)
  ;[1 1 1] Set off trail
  (`ActorComponent.Activate` (`self.Trail_Emitter_System`) false)
  (`KismetSystemLibrary.K2_SetTimerDelegate` (delegate `Thrust`) 0.01 true)
  (set `RotatingMovementComponent.RotationRate` (`KismetMathLibrary.MakeRotator` (`KismetMathLibrary.RandomFloatInRange` -20.0 20.0) 0.0 140.0) (`self.RotatingMovement`))
  (`KismetSystemLibrary.Delay` (/ (`self.Distance`) (`self.Speed`)))
  (`NiagaraComponent.SetVariableVec3` (`self.Niagara`) "ConeAngle" (`SceneComponent.GetForwardVector` (`self.RocketFoward`)))
  (`GameplayStatics.PlaySoundAtLocation` (`self.Explosion Sound`) (`self.K2_GetActorLocation`) (struct) (`self.Volume Multiplier Explosion`) (`KismetMathLibrary.RandomFloatInRange` 0.7 1.3) 0.0 "/Game/ModularFireworks2/BackEnd/Niagara/Sound/Att_Firework.Att_Firework" null null null)
  (`KismetSystemLibrary.DelayUntilNextTick`)
  (set `self.Speed` 0.0)
  (`SceneComponent.SetVisibility` (`self.Rocket`) false false)
  (`ActorComponent.SetActive` (`self.RotatingMovement`) false false)
  (`ActorComponent.SetActive` (`self.Trail_Emitter_System`) false false)
  (`ActorComponent.SetActive` (`self.Niagara`) true false)
  (if (>= _smoke_lifetime _trail_smoke_lifetime)
    (`KismetSystemLibrary.Delay` _smoke_lifetime)
    (else
      (`KismetSystemLibrary.Delay` _trail_smoke_lifetime)))
  (`self.K2_DestroyActor`))

(event `Thrust`
  ;[1 1 1] Movement
  (`SceneComponent.K2_AddWorldOffset` (`self.Rocket`) (* (`SceneComponent.GetForwardVector` (`self.RocketFoward`)) (* (`self.Speed`) 10.0)) false false))

(event `Test`
  ;[1 1 1] Test button
  (`SceneComponent.K2_SetWorldLocation` (`self.Niagara`) (+ (`SceneComponent.K2_GetComponentLocation` (`self.Rocket`)) (0.0 0.0 1500.0)) false false)
  (`ActorComponent.Activate` (`self.Niagara`) true))

(event `RandomColour`
  (`/Engine/EditorBlueprintResources/StandardMacros.FlipFlop`
    (:`A`
      (set `self.Colour` (make `LinearColor` (`KismetMathLibrary.RandomFloatInRange` 0.0 1.0) (`KismetMathLibrary.RandomFloatInRange` 0.0 1.0) 0.0 1.0)))
    (:`B`
      (`/Engine/EditorBlueprintResources/StandardMacros.FlipFlop`
        (:`A`
          (set `self.Colour` (make `LinearColor` 0.0 (`KismetMathLibrary.RandomFloatInRange` 0.0 1.0) (`KismetMathLibrary.RandomFloatInRange` 0.0 1.0) 1.0)))
        (:`B`
          (set `self.Colour` (make `LinearColor` (`KismetMathLibrary.RandomFloatInRange` 0.0 1.0) 0.0 (`KismetMathLibrary.RandomFloatInRange` 0.0 1.0) 1.0)))))))

(fn `UserConstructionScript`
  (bind _niagara (`self.Niagara`))
  (bind _niagara_2 (`self.Niagara`))
  (bind _niagara_3 (`self.Niagara`))
  (bind _niagara_4 (`self.Niagara`))
  (bind _trail_emitter_system (`self.Trail_Emitter_System`))
  (bind _returnvalue (* (`self.Size of Explosion`) 1000.0))
  ;[1 1 1] Select system
  (switch `/Game/ModularFireworks2/BackEnd/Niagara/ENums/E_System` (`self.System`)
    (:`NewEnumerator0`
      (`NiagaraComponent.SetAsset` _niagara_4 "/Game/ModularFireworks2/BackEnd/Niagara/Systems/System_PeonyPerfect.System_PeonyPerfect" true))
    (:`NewEnumerator1`
      (`NiagaraComponent.SetAsset` _niagara_4 "/Game/ModularFireworks2/BackEnd/Niagara/Systems/System_PeonyDefault.System_PeonyDefault" true))
    (:`NewEnumerator2`
      (`NiagaraComponent.SetAsset` _niagara_4 "/Game/ModularFireworks2/BackEnd/Niagara/Systems/System_AngledPeony.System_AngledPeony" true)
      ;[1 1 1] Set cone angle for firework
      (`NiagaraComponent.SetVariableVec3` (`self.Niagara`) "ConeAngle" (`SceneComponent.GetForwardVector` (`self.RocketFoward`)))))
  (`|ExecutionSequence`
    (:`then_0`
      ;[1 1 1] Explosion Variables
      (if (== (`self.Brightness`) 0.0)
        (set `self.DoesRenderLight` false))
      (`NiagaraComponent.SetNiagaraVariableBool` (`self.Niagara`) "DoesRenderLight" (`self.DoesRenderLight`))
      (`NiagaraComponent.SetVariableLinearColor` (`self.Niagara`) "CustomColor" (`self.Colour`))
      (`NiagaraComponent.SetVariableFloat` (`self.Niagara`) "Alpha" (`self.Brightness`))
      (`NiagaraComponent.SetVariableFloat` (`self.Niagara`) "NumOfParticles" (`KismetMathLibrary.Conv_IntToDouble` (/ (* (`self.Number Of Particles`) 5) 6)))
      (`NiagaraComponent.SetVariableFloat` _niagara "ParticleSize" (`self.Particle Size`))
      (`NiagaraComponent.SetVariableFloat` _niagara "ParticleLifetime" (`self.Particle Lifetime`))
      (`NiagaraComponent.SetVariableFloat` _niagara "Size" _returnvalue)
      ;;[1 0 0.0384] Smoke Variables
      (if (`self.Has Smoke`)
        (`NiagaraComponent.SetVariableFloat` _niagara_2 "SmokeSpawn" (* _returnvalue (/ (`self.Smoke Amount`) 100.0)))
        (else
          (`NiagaraComponent.SetVariableFloat` _niagara_2 "SmokeSpawn" 0.0)))
      (`NiagaraComponent.SetNiagaraVariableBool` (`self.Niagara`) "Has Variation" (`self.Has Scale Colour`))
      (`NiagaraComponent.SetVariableFloat` (`self.Niagara`) "Scale Colour Amount" (`self.Scale Colour Amount`)))
    (:`then_1`
      ;[1 0 0.007701] Smoke Variables
      (if (`self.Has Smoke`)
        (`NiagaraComponent.SetVariableFloat` _niagara_3 "SmokeSpawn" (* _returnvalue (/ (`self.Smoke Amount`) 50.0)))
        (else
          (`NiagaraComponent.SetVariableFloat` _niagara_3 "SmokeSpawn" 0.0)
          (set `self.Smoke Amount` 0.0)))
      (`NiagaraComponent.SetVariableFloat` (`self.Niagara`) "SmokeSize" (* (`self.Smoke Size`) 2.0))
      (`NiagaraComponent.SetVariableFloat` (`self.Niagara`) "SmokeLifetime" (`self.Smoke Lifetime`)))
    (:`then_2`
      (`NiagaraComponent.SetVariableFloat` (`self.Trail_Emitter_System`) "Trail Length" (`self.Trail Length`))
      (if (`self.Does Match Explosion Colour`)
        ;[1 1 1] Trail Variables
        (bind _output_get (set `self.TrailColour` (`self.Colour`)))
        (`NiagaraComponent.SetVariableLinearColor` (`self.Trail_Emitter_System`) "TrailColour" _output_get)
        (else
          (`NiagaraComponent.SetVariableLinearColor` (`self.Trail_Emitter_System`) "TrailColour" (`self.TrailColour`))))
      (if (`self.Has Trail Smoke`)
        (`NiagaraComponent.SetVariableFloat` _trail_emitter_system "TrailSmokeLifetime" (`self.Trail Smoke Lifetime`))
        (else
          (`NiagaraComponent.SetVariableFloat` (`self.Trail_Emitter_System`) "TrailSmokeLifetime" 0.0)
          (set `self.Trail Smoke Amount` 0.0)))
      (`NiagaraComponent.SetVariableFloat` _trail_emitter_system "TrailSpawnRate" (`self.Trail Spawn Rate`))
      (`NiagaraComponent.SetVariableBool` (`self.Trail_Emitter_System`) "DoesRenderLight" (`self.Does Render Light`))
      (`NiagaraComponent.SetVariableFloat` (`self.Trail_Emitter_System`) "TrailSmokeAmount" (`self.Trail Smoke Amount`)))))